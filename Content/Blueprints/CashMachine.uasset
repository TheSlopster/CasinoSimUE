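; CashMachine is an interactable Blueprint that pays the player a random amount of money.
; Any actor overlap toggles an in-range flag and adds or removes the CashMachineUI widget.
; Tick polls the player's IsInteracting flag and, while in range, adds the random amount to Money and plays a sound.
; The payout has no cooldown, so it repeats every frame while both flags hold.
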(event Custom|InteractedWith
  ;[0.125 0.125 0.125] Interacted With
  (bind _asplayer (Utilities|Casting|CastToPlayer (Game|GetPlayerCharacter 0)))
  (if (Variables|/Game/Blueprints/Player.Player_C|GetIsInteracting? _asplayer)
    (if (Variables|Default|GetIsInRange?)
      (Variables|Default|SetRandomNumber (Math|Random|RandomIntegerinRange 50 100))
      (Variables|/Game/Blueprints/Player.Player_C|SetMoney _asplayer (+ (Variables|Default|GetRandomNumber) (Variables|/Game/Blueprints/Player.Player_C|GetMoney _asplayer)))
      (Audio|PlaySound2D "/Game/Audio/MoneyGained.MoneyGained" 1.0 1.0 0.0 0 0))))

(event Custom|UI
  ;[0.1094 0.1094 0.1094] Create Widget
  (if (Variables|Default|GetIsInRange?)
    (bind _returnvalue (UserInterface|CreateWidget "/Game/UI/CashMachineUI.CashMachineUI_C"))
    (UserInterface|Viewport|AddtoViewport _returnvalue 0)
    (else
      (Widget|RemovefromParent _returnvalue))))

(event EventBeginPlay)

(event Collision|EventActorBeginOverlap
  (params (OtherActor :type Actor%20Object%20Reference))
  (Variables|Default|SetIsInRange? true)
  (CallFunction|UI))

(event Collision|EventActorEndOverlap
  (params (OtherActor :type Actor%20Object%20Reference))
  (Variables|Default|SetIsInRange? false)
  (CallFunction|UI))

(event EventTick
  (params (DeltaSeconds :type Float%20%28single-precision%29))
  (CallFunction|Interactedwith))

(fn ConstructionScript)