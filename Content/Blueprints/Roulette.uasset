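; Roulette gambling machine actor that charges the Player its use cost for a spin and pays triple on a win.
; Overlap toggles an on-screen UI, while Tick polls the player's interact flag when the machine is in range and usable.
; A spin locks the machine, plays sound and waits before a random roll decides the roughly one-in-four win.
; The result plays win or buzz audio, briefly flashing a widget on wins.
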(event Custom|InteractedWith
  ;[0.1146 0.1146 0.1146] Action When Interacted
  (bind _asplayer (Utilities|Casting|CastToPlayer (Game|GetPlayerCharacter 0)))
  (if (Variables|/Game/Blueprints/Player.Player_C|GetIsInteracting? _asplayer)
    (if (Variables|Default|GetIsUsable?)
      (if (Variables|Default|GetIsInRange?)
        (Variables|Default|SetIsUsable? false)
        (Variables|Default|SetRandomNumber (Math|Random|RandomIntegerinRange 0 100))
        (bind _asplayer_2 (Utilities|Casting|CastToPlayer (Game|Player|GetPlayerPawn 0)))
        (Variables|/Game/Blueprints/Player.Player_C|SetMoney _asplayer_2 (- (Variables|/Game/Blueprints/Player.Player_C|GetMoney _asplayer_2) (Variables|Default|GetCostToUse)))
        (Audio|SpawnSoundatLocation "/Game/Audio/Roulette_Spin.Roulette_Spin" (Transformation|GetActorLocation) "0, 0, 0" 1.0 1.0 0.0 "/Game/Audio/RouletteAttenuator.RouletteAttenuator" 0)
        (Utilities|FlowControl|Delay 16.0)
        (CallFunction|PlayerWonCheck)))))

(event Custom|PlayerWonCheck
  ;[0.09896 0.09896 0.09896] Check if Player Has Won and Give Money
  (if (<= (Variables|Default|GetRandomNumber) 25)
    (Variables|Default|SetWon? true)
    (bind _asplayer (Utilities|Casting|CastToPlayer (Game|Player|GetPlayerPawn 0)))
    (Variables|/Game/Blueprints/Player.Player_C|SetMoney _asplayer (+ (Variables|/Game/Blueprints/Player.Player_C|GetMoney _asplayer) (* (Variables|Default|GetCostToUse) 3)))
    (Variables|/Game/Blueprints/Player.Player_C|SetWinnings _asplayer (+ (Variables|/Game/Blueprints/Player.Player_C|GetMoney _asplayer) (* (Variables|Default|GetCostToUse) 3)))
    (Variables|Default|SetIsUsable? true)
    (Audio|SpawnSoundatLocation "/Game/Audio/Roulette-Horse-Win.Roulette-Horse-Win" (Transformation|GetActorLocation) "0, 0, 0" 1.0 1.0 0.0 "/Game/Audio/RouletteAttenuator.RouletteAttenuator" 0)
    (bind _returnvalue (UserInterface|CreateWidget "/Game/UI/WIN.WIN_C"))
    (UserInterface|Viewport|AddtoViewport _returnvalue 0)
    (Utilities|FlowControl|Delay 0.2)
    (Widget|RemovefromParent _returnvalue)
    (else
      (Variables|Default|SetWon? false)
      (Variables|Default|SetIsUsable? true)
      (Audio|SpawnSoundatLocation "/Game/Audio/Buzz.Buzz" (Transformation|GetActorLocation) "0, 0, 0" 1.0 1.0 0.0 "/Game/Audio/RouletteAttenuator.RouletteAttenuator" 0))))

(event Custom|UICheck
  ;[0.1094 0.1094 0.1094] Create Widget
  (if (Variables|Default|GetIsInRange?)
    (bind _returnvalue (UserInterface|CreateWidget "/Game/UI/Roulette1UI.Roulette1UI_C"))
    (UserInterface|Viewport|AddtoViewport _returnvalue 0)
    (else
      (Widget|RemovefromParent _returnvalue))))

(event EventBeginPlay
  (bind _asplayer (Utilities|Casting|CastToPlayer (Game|Player|GetPlayerPawn 0)))
  (Variables|/Game/Blueprints/Player.Player_C|SetCost _asplayer (Variables|Default|GetCostToUse)))

(event Collision|EventActorBeginOverlap
  (params (OtherActor :type Actor%20Object%20Reference))
  (Variables|Default|SetIsInRange? true)
  (CallFunction|UICheck))

(event EventTick
  (params (DeltaSeconds :type Float%20%28single-precision%29))
  (CallFunction|Interactedwith))

(event Collision|EventActorEndOverlap
  (params (OtherActor :type Actor%20Object%20Reference))
  (Variables|Default|SetIsInRange? false)
  (CallFunction|UICheck))

(fn ConstructionScript)